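; BP_Mayor is the city-management decision maker that earns income and spends each turn performing a chain of actions.
; TakeTurn banks population plus functional income-building revenue, then loops recalculating metrics and calling PerformBestAction (not defined here) until it returns none or a save-money action, returning the action names.
; Speculative metrics sum residential capacity and all income buildings, including non-functional ones.
; A Test event runs a single evaluate-and-act step.
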(event Custom|Test
  (CallFunction|CalculateMetrics)
  (Class|UtilityController|PerformBestAction))

(fn ConstructionScript)

(fn TakeTurn
  (CallFunction|CalculateIncome)
  (Utilities|Array|Clear (Variables|Default|GetActionsTaken))
  (CallFunction|CalculateMetrics :!label _label)
  (bind _returnvalue (Class|UtilityController|PerformBestAction))
  (if (and (not (== _returnvalue 0)) (not (== (Utilities|GetClass _returnvalue) "/Game/Mayor/Actions/BP_SaveMoneyAction.BP_SaveMoneyAction_C"))) ; If an action was performed and its not saving
    (Utilities|Array|Add (Variables|Default|GetActionsTaken) (Variables|/Script/AIAndGamesJam2021.UtilityAction|GetActionName _returnvalue))
    (goto _label)
    (else
      (return (Variables|Default|GetActionsTaken)))))

(fn CalculateMetrics
  (Variables|Default|SetSpeculativePopulationCap 0)
  (bind _outactors (Actor|GetAllActorsOfClass "/Game/Building/BP_ResidentialBuilding.BP_ResidentialBuilding_C"))
  (for _array_element _outactors
    (Variables|Default|SetSpeculativePopulationCap (+ (Variables|/Game/Building/BP_ResidentialBuilding.BP_ResidentialBuilding_C|GetPeople _array_element) (Variables|Default|GetSpeculativePopulationCap))))
  (Variables|Default|SetSpeculativeIncome (Variables|/Game/BP_CityManager.BP_CityManager_C|GetPopulation (.AsBP%20City%20Manager (Utilities|Casting|CastToBP_CityManager (Game|GetGameMode)))))
  (bind _outactors_2 (Actor|GetAllActorsOfClass "/Game/Building/BP_IncomeBuilding.BP_IncomeBuilding_C"))
  (for _array_element_2 _outactors_2
    (Variables|Default|SetSpeculativeIncome (+ (Variables|/Game/Building/BP_IncomeBuilding.BP_IncomeBuilding_C|GetIncome _array_element_2) (Variables|Default|GetSpeculativeIncome)))))

(fn CalculateIncome
  (LocalVariables|SetIncome (Variables|/Game/BP_CityManager.BP_CityManager_C|GetPopulation (.AsBP%20City%20Manager (Utilities|Casting|CastToBP_CityManager (Game|GetGameMode)))))
  (bind _outactors (Actor|GetAllActorsOfClass "/Game/Building/BP_IncomeBuilding.BP_IncomeBuilding_C"))
  (for _array_element _outactors
    (if (Variables|/Game/Building/BP_Building.BP_Building_C|GetbFunctional _array_element)
      (LocalVariables|SetIncome (+ (Variables|/Game/Building/BP_IncomeBuilding.BP_IncomeBuilding_C|GetIncome _array_element) (LocalVariables|GetIncome)))))
  (Variables|Default|SetMoney (+ (LocalVariables|GetIncome) (Variables|Default|GetMoney))))