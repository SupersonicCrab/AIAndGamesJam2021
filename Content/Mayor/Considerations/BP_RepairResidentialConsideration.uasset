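; Utility-style consideration for the Mayor, named for the decision to repair residential buildings.
; GetConsideration reads the current and maximum population from BP_CityManager, the game mode, and returns them as floats in an X/Y pair.
; It does no scoring itself: the Controller input is ignored and the X / Y math expression is unused.
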(fn ConstructionScript)

(fn GetConsideration
  (params (Controller :type Utility%20Controller%20Object%20Reference))
  (bind _returnvalue (Game|GetGameMode))
  (bind _asbp_city_manager (Utilities|Casting|CastToBP_CityManager _returnvalue))
  (return (|(x/y) (Math|Conversions|ToFloat(Integer) (Variables|/Game/BP_CityManager.BP_CityManager_C|GetPopulation _asbp_city_manager)) (Math|Conversions|ToFloat(Integer) (Variables|/Game/BP_CityManager.BP_CityManager_C|GetMaxPopulation _asbp_city_manager)))))