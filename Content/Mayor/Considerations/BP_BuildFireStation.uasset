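; Mayor AI consideration that scores how much a new fire station is needed.
; GetConsideration counts burning BP_Building actors and existing BP_FireStation actors across the level.
; It weights fires against stations, each station offsetting two fires, and returns the squared difference.
; Squaring discards the sign, so a surplus of stations also yields a positive score.
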(fn ConstructionScript)

(fn GetConsideration
  (params (Controller :type Utility%20Controller%20Object%20Reference))
  (bind _outactors (Actor|GetAllActorsOfClass "/Game/Building/BP_Building.BP_Building_C"))
  (for _array_element _outactors
    (if (Variables|/Game/Building/BP_Building.BP_Building_C|GetbBurning _array_element)
      (Math|Float|IncrementFloat (LocalVariables|GetBurningBuildings))))
  (bind _outactors_2 (Actor|GetAllActorsOfClass "/Game/Building/BP_FireStation.BP_FireStation_C"))
  (return (Math|Float|Power (|((x*0.050000)-(y*0.100000)) (LocalVariables|GetBurningBuildings) (Math|Conversions|ToFloat(Integer) (Utilities|Array|Length _outactors_2))) 2.0)))