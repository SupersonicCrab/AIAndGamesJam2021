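; BP_SaveMoneyConsideration2 is a consideration for the Mayor that scores how much it needs to save money.
; It sums Income from every BP_IncomeBuilding that is neither mob-controlled nor flagged Functional.
; That total is added to the Mayor's Money, normalized against a fixed range and inverted, so the score rises as available funds shrink.
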(fn ConstructionScript)

(fn GetConsideration
  (params (Controller :type Utility%20Controller%20Object%20Reference))
  (bind _outactors (Actor|GetAllActorsOfClass "/Game/Building/BP_IncomeBuilding.BP_IncomeBuilding_C"))
  (for _array_element _outactors
    (if (and (not (Variables|/Game/Building/BP_IncomeBuilding.BP_IncomeBuilding_C|GetbMobControlled _array_element)) (not (Variables|/Game/Building/BP_Building.BP_Building_C|GetbFunctional _array_element)))
      (LocalVariables|SetTotalIncome (+ (LocalVariables|GetTotalIncome) (Variables|/Game/Building/BP_IncomeBuilding.BP_IncomeBuilding_C|GetIncome _array_element)))))
  (return (- 1.0 (Math|Float|NormalizetoRange (Math|Conversions|ToFloat(Integer) (+ (Variables|/Game/Mayor/BP_Mayor.BP_Mayor_C|GetMoney (.AsBP%20Mayor (Utilities|Casting|CastToBP_Mayor Controller))) (LocalVariables|GetTotalIncome))) 0.0 3e+03))))