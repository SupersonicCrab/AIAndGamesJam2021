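; AI consideration for the mayor that scores how much clearing rubble matters, based on the plots remaining.
; It counts every BP_Building whose Difficulty is at or below the current Difficulty of the BP_CityManager game mode.
; A math expression turns that count into the returned score, labelled as double the count, or zero when none qualify.
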(fn GetConsideration
  (params (Controller :type Utility%20Controller%20Object%20Reference))
  (bind _outactors (Actor|GetAllActorsOfClass "/Game/Building/BP_Building.BP_Building_C"))
  (for _array_element _outactors
    (if (<= (Variables|/Game/Building/BP_Building.BP_Building_C|GetDifficulty _array_element) (Variables|/Game/BP_CityManager.BP_CityManager_C|GetDifficulty (.AsBP%20City%20Manager (Utilities|Casting|CastToBP_CityManager (Game|GetGameMode)))))
      (Math|Float|IncrementFloat (LocalVariables|GetPlotsRemaining))))
  (if (not (== (LocalVariables|GetPlotsRemaining) 0.0))
    (return (|(2/x) (LocalVariables|GetPlotsRemaining)))
    (else
      (return 0.0))))

(fn ConstructionScript)