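; Utility-style consideration that scores the mayor's repair choice from city happiness.
; GetConsideration reads Happiness from BP_CityManager, the game mode, and ignores the passed Controller.
; A math expression maps it through an inverted half sine wave offset upward.
; Assuming a 0–100 happiness scale, the score is highest at both extremes (1.5) and lowest at the midpoint (0.5).
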(fn ConstructionScript)

(fn GetConsideration
  (params (Controller :type Utility%20Controller%20Object%20Reference))
  (return (|((sin((pi+((x/100)*pi))))+1.500000) (Math|Trig|GetPI) (Math|Conversions|ToFloat(Integer) (Variables|/Game/BP_CityManager.BP_CityManager_C|GetHappiness (.AsBP%20City%20Manager (Utilities|Casting|CastToBP_CityManager (Game|GetGameMode))))))))