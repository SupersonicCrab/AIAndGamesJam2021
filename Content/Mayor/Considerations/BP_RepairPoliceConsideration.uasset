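; Utility consideration for the mayor AI that scores how much repairing police stations matters.
; It counts functional police stations and reads city happiness from the city manager game mode, normalized to a unit range.
; Happiness plus a weighted station count feeds an inverse-square curve, clamped between half and full score.
; The score stays at maximum until that sum exceeds one, then falls toward the floor.
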(fn ConstructionScript)

(fn GetConsideration
  (params (Controller :type Utility%20Controller%20Object%20Reference))
  (bind _outactors (Actor|GetAllActorsOfClass "/Game/Building/BP_PoliceStation.BP_PoliceStation_C"))
  (for _array_element _outactors
    (if (Variables|/Game/Building/BP_Building.BP_Building_C|GetbFunctional _array_element)
      (Math|Integer|IncrementInt (LocalVariables|GetActivePoliceStations))))
  (return (Math|Float|Clamp(Float) (Math|Float|Power (|(x+(0.100000*y)) (Math|Float|NormalizetoRange (Math|Conversions|ToFloat(Integer) (Variables|/Game/BP_CityManager.BP_CityManager_C|GetHappiness (.AsBP%20City%20Manager (Utilities|Casting|CastToBP_CityManager (Game|GetGameMode))))) 0.0 1e+02) (Math|Conversions|ToFloat(Integer) (LocalVariables|GetActivePoliceStations))) -2.0) 0.5)))