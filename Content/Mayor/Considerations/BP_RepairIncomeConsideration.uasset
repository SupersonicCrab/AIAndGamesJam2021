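; Mayor AI consideration that scores repairing income buildings from the income of broken versus working ones.
; GetConsideration scans every BP_IncomeBuilding, skips mob-controlled ones, and sums Income by Functional state.
; The variable names read inverted: non-functional buildings add to TotalIncome, functional ones to LostIncome.
; Their difference feeds a math expression built on the constants 250 and 0.5 to give the returned score.
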(fn ConstructionScript)

(fn GetConsideration
  (params (Controller :type Utility%20Controller%20Object%20Reference))
  (bind _outactors (Actor|GetAllActorsOfClass "/Game/Building/BP_IncomeBuilding.BP_IncomeBuilding_C"))
  (for _array_element _outactors
    (if (not (Variables|/Game/Building/BP_IncomeBuilding.BP_IncomeBuilding_C|GetbMobControlled _array_element))
      (if (not (Variables|/Game/Building/BP_Building.BP_Building_C|GetbFunctional _array_element))
        (LocalVariables|SetTotalIncome (+ (LocalVariables|GetTotalIncome) (Variables|/Game/Building/BP_IncomeBuilding.BP_IncomeBuilding_C|GetIncome _array_element)))
        (else
          (LocalVariables|SetLostIncome (+ (LocalVariables|GetLostIncome) (Variables|/Game/Building/BP_IncomeBuilding.BP_IncomeBuilding_C|GetIncome _array_element)))))))
  (return (|((250/x)+0.500000) (Math|Conversions|ToFloat(Integer) (- (LocalVariables|GetTotalIncome) (LocalVariables|GetLostIncome))))))