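; BP_RepairResidential is a Mayor action that pays to repair a damaged residential building.
; IsActionPossible scans all residential buildings and stores the first that is non-functional, not burning and repairable for half its build price with the Mayor's money.
; PerformAction deducts that cost from the Mayor and flags the stored building as Repairing.
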(fn ConstructionScript)

(fn IsActionPossible
  (params (Controller :type Utility%20Controller%20Object%20Reference))
  (bind _outactors (Actor|GetAllActorsOfClass "/Game/Building/BP_ResidentialBuilding.BP_ResidentialBuilding_C"))
  (bind _array_element (Utilities|Array|ForEachLoopwithBreak _outactors :!label _label)
    (:LoopBody
      (if (and (not (Variables|/Game/Building/BP_Building.BP_Building_C|GetbFunctional _array_element)) (not (Variables|/Game/Building/BP_Building.BP_Building_C|GetbBurning _array_element)))
        (if (>= (Variables|/Game/Mayor/BP_Mayor.BP_Mayor_C|GetMoney (.AsBP%20Mayor (Utilities|Casting|CastToBP_Mayor Controller))) (/ (Variables|/Game/Building/BP_Building.BP_Building_C|GetBuildPrice _array_element) 2))
          (Variables|Default|SetResidentialBuilding _array_element)
          (goto _label Break))))
    (:Completed
      (return (== (Variables|Default|GetResidentialBuilding) 0)))))

(fn PerformAction
  (params (Controller :type Utility%20Controller%20Object%20Reference))
  (bind _asbp_mayor (Utilities|Casting|CastToBP_Mayor Controller))
  (bind _residentialbuilding (Variables|Default|GetResidentialBuilding))
  (Variables|/Game/Mayor/BP_Mayor.BP_Mayor_C|SetMoney _asbp_mayor (- (Variables|/Game/Mayor/BP_Mayor.BP_Mayor_C|GetMoney _asbp_mayor) (/ (Variables|/Game/Building/BP_Building.BP_Building_C|GetBuildPrice _residentialbuilding) 2)))
  (Variables|/Game/Building/BP_Building.BP_Building_C|SetbRepairing _residentialbuilding true)
  (return true))