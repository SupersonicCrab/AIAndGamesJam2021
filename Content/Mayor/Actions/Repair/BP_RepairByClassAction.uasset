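; BP_RepairByClassAction is a mayor action that repairs a broken building of a configured class.
; Its possibility check scans all actors of that class for the first completed, non-burning, non-functional one the mayor can afford at half its build price, and caches it.
; Performing the action deducts that half price from the mayor's money and flags the cached building as repairing.
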(fn ConstructionScript)

(fn IsActionPossible
  (params (Controller :type Utility%20Controller%20Object%20Reference))
  (bind _outactors (Actor|GetAllActorsOfClass (Variables|Default|GetBuildingClass)))
  (bind _array_element (Utilities|Array|ForEachLoopwithBreak _outactors :!label _label)
    (:LoopBody
      (if (Math|Boolean|ANDBoolean (not (Variables|/Game/Building/BP_Building.BP_Building_C|GetbFunctional _array_element)) (not (Variables|/Game/Building/BP_Building.BP_Building_C|GetbBurning _array_element)) (== (Variables|/Game/Building/BP_Building.BP_Building_C|GetBuildProgress _array_element) 100))
        (if (>= (Variables|/Game/Mayor/BP_Mayor.BP_Mayor_C|GetMoney (.AsBP%20Mayor (Utilities|Casting|CastToBP_Mayor Controller))) (/ (Variables|/Game/Building/BP_Building.BP_Building_C|GetBuildPrice _array_element) 2))
          (Variables|Default|SetBuilding _array_element)
          (goto _label Break))))
    (:Completed
      (return (!= (Variables|Default|GetBuilding) 0)))))

(fn PerformAction
  (params (Controller :type Utility%20Controller%20Object%20Reference))
  (bind _asbp_mayor (Utilities|Casting|CastToBP_Mayor Controller))
  (bind _building (Variables|Default|GetBuilding))
  (Variables|/Game/Mayor/BP_Mayor.BP_Mayor_C|SetMoney _asbp_mayor (- (Variables|/Game/Mayor/BP_Mayor.BP_Mayor_C|GetMoney _asbp_mayor) (/ (Variables|/Game/Building/BP_Building.BP_Building_C|GetBuildPrice _building) 2)))
  (Variables|/Game/Building/BP_Building.BP_Building_C|SetbRepairing _building true)
  (return true))