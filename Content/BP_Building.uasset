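; BP_Building is a building Blueprint with construction progress driven by a BuildingEvent function.
; Each call adds BuildRate to BuildProgress while it is below 100, with no clamp on the final step.
; An unconnected check for repairing while Health is below 100 is present but unused, and the construction script is empty.
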(fn ConstructionScript)

(fn BuildingEvent
  (if (< (Variables|Default|GetBuildProgress) 100)
    (Variables|Default|SetBuildProgress (+ (Variables|Default|GetBuildProgress) (Variables|Default|GetBuildRate)))))