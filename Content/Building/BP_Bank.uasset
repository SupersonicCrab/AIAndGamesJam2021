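; BP_Bank is a bank building in a city game where the player balances money, mob trust and council suspicion.
; MobInteraction adds the bank's Income, MobTrust and CouncilSuspicion values to the matching totals on the BP_CityManager game mode, then refreshes the UI.
; The construction script only calls its parent, and the BeginPlay parent call is disabled.
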(fn ConstructionScript
  (|CallParentFunction))

(fn MobInteraction
  (bind _returnvalue (Game|GetGameMode))
  (bind _asbp_city_manager (Utilities|Casting|CastToBP_CityManager _returnvalue))
  (Variables|/Game/BP_CityManager.BP_CityManager_C|SetPlayerMoney _asbp_city_manager (+ (Variables|/Game/BP_CityManager.BP_CityManager_C|GetPlayerMoney _asbp_city_manager) (Variables|Default|GetIncome)))
  (Variables|/Game/BP_CityManager.BP_CityManager_C|SetMobTrust _asbp_city_manager (+ (Variables|/Game/BP_CityManager.BP_CityManager_C|GetMobTrust _asbp_city_manager) (Variables|Default|GetMobTrust)))
  (Variables|/Game/BP_CityManager.BP_CityManager_C|SetCouncilSuspicion _asbp_city_manager (+ (Variables|/Game/BP_CityManager.BP_CityManager_C|GetCouncilSuspicion _asbp_city_manager) (Variables|Default|GetCouncilSuspicion)))
  (Default|UpdateUI _asbp_city_manager))