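; Police station building for the city-builder that can stage random raids on mob hangouts, raising happiness while shrinking the population.
; BuildingEvent runs the parent logic, then, if the building is functional, rolls against RaidChance.
; A raid updates Happiness and Population on BP_CityManager, with the loss clamped using the unemployed count, then posts a ranked alert through the player controller's overlay.
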(event EventBeginPlay)

(event Collision|EventActorBeginOverlap
  (params (OtherActor :type Actor%20Object%20Reference)))

(event EventTick
  (params (DeltaSeconds :type Float%20%28single-precision%29)))

(fn ConstructionScript
  (|CallParentFunction))

(fn BuildingEvent
  (bind _returnvalue (Game|GetGameMode))
  (bind _raidunemployeddecrease (Variables|Default|GetRaidUnemployedDecrease))
  (bind _asbp_city_manager (Utilities|Casting|CastToBP_CityManager _returnvalue))
  (|CallParentFunction)
  (if (Variables|Default|GetbFunctional)
    (if (>= (Variables|Default|GetRaidChance) (Math|Random|RandomIntegerinRange 0 100)) ; If raid a happens this turn
      (Variables|/Game/BP_CityManager.BP_CityManager_C|SetHappiness _asbp_city_manager (+ (Variables|/Game/BP_CityManager.BP_CityManager_C|GetHappiness _asbp_city_manager) (Variables|Default|GetRaidHappinessIncrease))) ; Increase happiness
      (Variables|/Game/BP_CityManager.BP_CityManager_C|SetPopulation _asbp_city_manager (- (Variables|/Game/BP_CityManager.BP_CityManager_C|GetPopulation _asbp_city_manager) (Math|Integer|Clamp(Integer) (- (- (Variables|/Game/BP_CityManager.BP_CityManager_C|GetPopulation _asbp_city_manager) (Variables|/Game/BP_CityManager.BP_CityManager_C|GetEmployedPopulation _asbp_city_manager)) _raidunemployeddecrease) 0 _raidunemployeddecrease))) ; Decrease population
      (Default|NewAlert (Variables|/Game/Player/BP_CityPlayerController.BP_CityPlayerController_C|GetOverlayRef (.AsBP%20City%20Player%20Controller (Utilities|Casting|CastToBP_CityPlayerController (Game|GetPlayerController 0)))) (Utilities|Struct|MakeFAlert "The police have raided one of the mob hangouts. -50 unemployed population, +10% happiness" "Police Raid" "/Game/UI/UI_Assets/MainMenu/T_Star.T_Star" "NewEnumerator2")))))