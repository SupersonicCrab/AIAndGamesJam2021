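; BP_FireStation is a city building that puts out fires and can be hit by a mob interaction.
; On its building event, if functional, it scans all BP_Building actors and extinguishes the first one found burning.
; MobInteraction drops its health to a fixed value, marks it repairing and non-functional, then adds its trust and suspicion values to BP_CityManager and refreshes the UI.
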(event EventBeginPlay)

(event Collision|EventActorBeginOverlap
  (params (OtherActor :type Actor%20Object%20Reference)))

(event EventTick
  (params (DeltaSeconds :type Float%20%28single-precision%29)))

(fn ConstructionScript
  (|CallParentFunction))

(fn MobInteraction
  (bind _returnvalue (Game|GetGameMode))
  (bind _asbp_city_manager (Utilities|Casting|CastToBP_CityManager _returnvalue))
  (Variables|Default|SetHealth 34)
  (Variables|Default|SetbRepairing true)
  (Variables|Default|SetbFunctional false)
  (Variables|/Game/BP_CityManager.BP_CityManager_C|SetMobTrust _asbp_city_manager (+ (Variables|/Game/BP_CityManager.BP_CityManager_C|GetMobTrust _asbp_city_manager) (Variables|Default|GetMobTrust)))
  (Variables|/Game/BP_CityManager.BP_CityManager_C|SetCouncilSuspicion _asbp_city_manager (+ (Variables|/Game/BP_CityManager.BP_CityManager_C|GetCouncilSuspicion _asbp_city_manager) (Variables|Default|GetCouncilSuspicion)))
  (Default|UpdateUI _asbp_city_manager))

(fn BuildingEvent
  (|CallParentFunction)
  (if (Variables|Default|GetbFunctional)
    (bind _outactors (Actor|GetAllActorsOfClass "/Game/Building/BP_Building.BP_Building_C"))
    (bind _array_element (Utilities|Array|ForEachLoopwithBreak _outactors :!label _label)
      (:LoopBody
        (if (Variables|/Game/Building/BP_Building.BP_Building_C|GetbBurning _array_element) ; If building is on fire
          (Variables|/Game/Building/BP_Building.BP_Building_C|SetbBurning _array_element false)
          (goto _label Break))))))