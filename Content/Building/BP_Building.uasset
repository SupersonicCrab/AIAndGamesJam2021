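; BP_Building is a building actor that can be constructed, repaired, set on fire and reduced to rubble.
; On BeginPlay it applies a mesh variation, picking one at random if none is set.
; Each BuildingEvent call advances one state by BuildRate: burning takes priority over construction, then repair, and the building is otherwise marked Functional.
; MobInteraction starts the fire, and zero health while burning spawns BP_Rubble and destroys the actor.
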(event EventBeginPlay
  (if (> (Utilities|Array|Length (Variables|Default|GetMeshVariations)) 0) ; If there are any mesh variations
    (if (== (Variables|Default|GetMeshVariation) -1) ; If a variation hasn't been picked
      (Variables|Default|SetMeshVariation (Math|Random|RandomIntegerinRange 0 (- (Utilities|Array|Length (Variables|Default|GetMeshVariations)) 1))))
    (Components|StaticMesh|SetStaticMesh (Variables|Default|GetBuildingMesh) (Utilities|Array|Get(acopy) (Variables|Default|GetMeshVariations) (Variables|Default|GetMeshVariation)))))

(fn ConstructionScript)

(fn BuildingEvent
  (if (Variables|Default|GetbBurning) ; If burning
    (Variables|Default|SetHealth (Math|Integer|Clamp(Integer) (- (Variables|Default|GetHealth) (Variables|Default|GetBuildRate)) 0 100)) ; Reduce health
    (Variables|Default|SetbFunctional false)
    (if (== (Variables|Default|GetHealth) 0) ; If health is 0
      (Game|SpawnActorfromClass "/Game/Building/BP_Rubble.BP_Rubble_C" (Transformation|GetActorTransform) "Undefined" 0 0) ; Replace with rubble
      (Actor|DestroyActor))
    (elif (< (Variables|Default|GetBuildProgress) 100) ; If not fully built
      (Variables|Default|SetBuildProgress (Math|Integer|Clamp(Integer) (+ (Variables|Default|GetBuildProgress) (Variables|Default|GetBuildRate)) 0 100)) ; Increase build progress
      (Variables|Default|SetbFunctional false)
      (elif (and (Variables|Default|GetbRepairing) (< (Variables|Default|GetHealth) 100)) ; If repairing
        (Variables|Default|SetHealth (Math|Integer|Clamp(Integer) (+ (Variables|Default|GetHealth) (Variables|Default|GetBuildRate)) 0 100)) ; Increase health
        (Variables|Default|SetbFunctional false)
        (else
          (Variables|Default|SetbFunctional true))))))

(fn MobInteraction
  (Variables|Default|SetbBurning true))