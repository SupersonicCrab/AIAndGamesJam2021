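; Player controller for the city game that creates the overlay UI, picks a named level camera by difficulty, and handles mouse interaction with buildings.
; Easy and Medium share MediumCamera, while Hard uses HardCamera.
; Tick traces under the cursor and rebuilds a tooltip widget every frame for buildings, skipping plots and adding mob-control state for income buildings.
; In targeting mode, left-click charges city manager money to trigger a building's mob interaction, or raises an alert.
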(event Custom|SpawnUI
  ;[1 1 1] Create overlay ui
  (bind _returnvalue (UserInterface|CreateWidget "/Game/UI/WBP_Overlay.WBP_Overlay_C"))
  (bind _output_get (Variables|Default|SetOverlayRef _returnvalue))
  (UserInterface|Viewport|AddtoPlayerScreen _output_get)
  (Variables|Default|SetbShowMouseCursor true)
  (Input|SetInputModeGameandUI self _returnvalue "DoNotLock" false)
  (CallFunction|SetupCamera))

(event Custom|SetupCamera
  ;[1 1 1] Setup which camera to use based on difficulty
  (switch Utilities|FlowControl|Switch|SwitchonEDifficulty (Variables|/Game/BP_CityManager.BP_CityManager_C|GetDifficulty (.AsBP%20City%20Manager (Utilities|Casting|CastToBP_CityManager (Game|GetGameMode))))
    (:NewEnumerator0
      (Variables|Default|SetCameraName "MediumCamera"))
    (:NewEnumerator1
      (Variables|Default|SetCameraName "MediumCamera"))
    (:NewEnumerator2
      (Variables|Default|SetCameraName "HardCamera")))
  (bind _outactors (Actor|GetAllActorsOfClass "/Script/Engine.CameraActor"))
  (bind _array_element (Utilities|Array|ForEachLoopwithBreak _outactors :!label _label)
    (:LoopBody
      (if (Utilities|Enum|Equal(Enum) (Utilities|GetObjectName _array_element) (Variables|Default|GetCameraName))
        (Variables|Default|SetSelectedCamera _array_element)
        (goto _label Break)))
    (:Completed
      (Game|Player|SetViewTargetwithBlend (Variables|Default|GetSelectedCamera) 0.0 "VTBlend_Linear" 0.0 false))))

(event EventTick
  (params (DeltaSeconds :type Float%20%28single-precision%29))
  (bind (_locationx _locationy) (Game|Player|GetMousePosition))
  (bind (_locationx_2 _locationy_2) (Game|Player|GetMousePosition))
  (bind (_worldlocation _worlddirection) (Game|Player|ConvertMouseLocationToWorldSpace))
  ;[1 1 1] Tooltip setup
  (Utilities|IsValid (Variables|Default|GetTooltipRef)
    (:Is%20Valid
      (Widget|RemovefromParent (Variables|Default|GetTooltipRef)))
    (:Is%20Not%20Valid
      _))
  (bind _outhit (Collision|LineTraceByChannel _worldlocation (+ _worldlocation (* _worlddirection 1e+08)) "TraceTypeQuery1" false 0 "None" true "(R=1.000000,G=0.000000,B=0.000000,A=1.000000)" "(R=0.000000,G=1.000000,B=0.000000,A=1.000000)" 1.0))
  (bind _asbp_income_building (Utilities|Casting|CastToBP_IncomeBuilding (.HitActor (Collision|BreakHitResult _outhit)))
    (:then
      (bind _returnvalue (UserInterface|CreateWidget "/Game/UI/WBP_Tooltip.WBP_Tooltip_C" 0 (Variables|/Game/Building/BP_Building.BP_Building_C|GetName _asbp_income_building) (Variables|/Game/Building/BP_Building.BP_Building_C|GetDescription _asbp_income_building) (Variables|/Game/Building/BP_Building.BP_Building_C|GetHealth _asbp_income_building) (Variables|/Game/Building/BP_Building.BP_Building_C|GetMobDescription _asbp_income_building) (Variables|/Game/Building/BP_Building.BP_Building_C|GetBuildProgress _asbp_income_building) (< (Variables|/Game/Building/BP_Building.BP_Building_C|GetBuildProgress _asbp_income_building) 100) (Variables|/Game/Building/BP_Building.BP_Building_C|GetbRepairing _asbp_income_building) (Variables|/Game/Building/BP_IncomeBuilding.BP_IncomeBuilding_C|GetbMobControlled _asbp_income_building) (Variables|/Game/Building/BP_Building.BP_Building_C|GetHealth _asbp_income_building) (Variables|/Game/Building/BP_Building.BP_Building_C|GetbBurning _asbp_income_building)))
      (UserInterface|Viewport|AddtoViewport _returnvalue 0)
      (Class|Widget|SetRenderTransform _returnvalue (Utilities|Struct|MakeWidgetTransform (Math|Vector2D|MakeVector2D (+ _locationx_2 1e+02) _locationy_2) "(X=1.000000,Y=1.000000)" "(X=0.000000,Y=0.000000)" 0.0))
      (Variables|Default|SetTooltipRef _returnvalue))
    (:CastFailed
      (bind _asbp_building (Utilities|Casting|CastToBP_Building (.HitActor (Collision|BreakHitResult _outhit))))
      (Utilities|Casting|CastToBP_Plot _asbp_building
        (:CastFailed
          (bind _returnvalue_2 (UserInterface|CreateWidget "/Game/UI/WBP_Tooltip.WBP_Tooltip_C" 0 (Variables|/Game/Building/BP_Building.BP_Building_C|GetName _asbp_building) (Variables|/Game/Building/BP_Building.BP_Building_C|GetDescription _asbp_building) (Variables|/Game/Building/BP_Building.BP_Building_C|GetHealth _asbp_building) (Variables|/Game/Building/BP_Building.BP_Building_C|GetMobDescription _asbp_building) (Variables|/Game/Building/BP_Building.BP_Building_C|GetBuildProgress _asbp_building) (< (Variables|/Game/Building/BP_Building.BP_Building_C|GetBuildProgress _asbp_building) 100) (Variables|/Game/Building/BP_Building.BP_Building_C|GetbRepairing _asbp_building) false (Variables|/Game/Building/BP_Building.BP_Building_C|GetHealth _asbp_building) (Variables|/Game/Building/BP_Building.BP_Building_C|GetbBurning _asbp_building)))
          (UserInterface|Viewport|AddtoViewport _returnvalue_2 0)
          (Class|Widget|SetRenderTransform _returnvalue_2 (Utilities|Struct|MakeWidgetTransform (Math|Vector2D|MakeVector2D (+ _locationx 1e+02) _locationy) "(X=1.000000,Y=1.000000)" "(X=0.000000,Y=0.000000)" 0.0))
          (Variables|Default|SetTooltipRef _returnvalue_2))))))

(event Input|MouseEvents|LeftMouseButton
  (params (Key :type Key%20Structure :default "None"))
  (bind (_worldlocation _worlddirection) (Game|Player|ConvertMouseLocationToWorldSpace))
  ;[1 1 1] Target building
  (:Pressed
    (if (Variables|Default|GetTargetting)
      (bind _outhit (Collision|LineTraceByChannel _worldlocation (+ _worldlocation (* _worlddirection 1e+08)) "TraceTypeQuery1" false 0 "ForDuration" true "(R=1.000000,G=0.000000,B=0.000000,A=1.000000)" "(R=0.000000,G=1.000000,B=0.000000,A=1.000000)" 1.0))
      (bind _asbp_building (Utilities|Casting|CastToBP_Building (.HitActor (Collision|BreakHitResult _outhit))))
      (bind _asbp_city_manager (Utilities|Casting|CastToBP_CityManager (Game|GetGameMode)))
      (if (>= (Variables|/Game/BP_CityManager.BP_CityManager_C|GetPlayerMoney _asbp_city_manager) 200)
        (Variables|/Game/BP_CityManager.BP_CityManager_C|SetPlayerMoney _asbp_city_manager (- (Variables|/Game/BP_CityManager.BP_CityManager_C|GetPlayerMoney _asbp_city_manager) 200))
        (Default|MobInteraction _asbp_building)
        (Variables|Default|SetTargetting false)
        (Default|UpdateUI _asbp_city_manager)
        (Default|UnlockPlayerActions (Variables|Default|GetOverlayRef))
        (else
          (Default|NewAlert (Variables|Default|GetOverlayRef) (Utilities|Struct|MakeFAlert "Targetting Buildings with the Mob requires $200" "Not Enough Money" "/Game/UI/UI_Assets/HappinessBois/T_Neutral.T_Neutral" "NewEnumerator0")))))))

(fn ConstructionScript)