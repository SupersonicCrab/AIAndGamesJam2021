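; BP_CityManager runs the city turn loop, alternating between the AI-style BP_Mayor turn and the player's turn.
; On BeginPlay it loads the difficulty from the save, caches the mayor and keeps buildings matching that difficulty.
; The mayor turn locks player actions on the overlay, logs the result, then unlocks them.
; SetupUI pushes happiness, mob trust and council suspicion to that overlay; random and building event phases are empty stubs.
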(event Custom|SetupUI
  (bind _returnvalue (Game|GetPlayerController 0))
  (bind _asbp_city_player_character (Utilities|Casting|CastToBP_CityPlayerCharacter _returnvalue))
  (bind _overlayref (Variables|/Game/Player/BP_CityPlayerCharacter.BP_CityPlayerCharacter_C|GetOverlayRef _asbp_city_player_character))
  (Default|UpdateHappiness _overlayref (Variables|Default|GetHappiness))
  (Default|UpdateMobTrust _overlayref (Variables|Default|GetMobTrust))
  (Default|UpdateCouncilStatus _overlayref (Variables|Default|GetCouncilSuspicion)))

(event Custom|StartMayorTurn
  (bind _returnvalue (Game|GetPlayerController 0))
  (bind _asbp_city_player_character (Utilities|Casting|CastToBP_CityPlayerCharacter _returnvalue))
  (bind _overlayref (Variables|/Game/Player/BP_CityPlayerCharacter.BP_CityPlayerCharacter_C|GetOverlayRef _asbp_city_player_character))
  (Default|LockPlayerActions _overlayref)
  (bind _actionstaken (Default|TakeTurn (Variables|Default|GetMayorRef)))
  (Default|UpdateCityLog _overlayref _actionstaken)
  (CallFunction|StartPlayerTurn))

(event Custom|DifficultySetup
  (bind _returnvalue (SaveGame|LoadGamefromSlot (Variables|Default|GetGameSaveSlot)))
  (bind _asbp_player_save (Utilities|Casting|CastToBP_PlayerSave _returnvalue))
  (Variables|Default|SetDifficulty (Variables|/Game/Player/BP_PlayerSave.BP_PlayerSave_C|GetDifficulty _asbp_player_save)))

(event Custom|StartPlayerTurn
  (Default|UnlockPlayerActions (Variables|/Game/Player/BP_CityPlayerCharacter.BP_CityPlayerCharacter_C|GetOverlayRef (.AsBP%20City%20Player%20Character (Utilities|Casting|CastToBP_CityPlayerCharacter (Game|GetPlayerController 0))))))

(event Custom|StartRandomEventPhase)

(event Custom|StartBuildingEventPhase)

(event EventBeginPlay
  (CallFunction|DifficultySetup)
  (bind _returnvalue (Actor|GetActorOfClass "/Game/Mayor/BP_Mayor.BP_Mayor_C"))
  (Variables|Default|SetMayorRef _returnvalue)
  (bind _outactors (Actor|GetAllActorsOfClass "/Game/Building/BP_Building.BP_Building_C")) ; Get all plots
  (bind _output_get (Variables|Default|SetAllBuildings _outactors))
  (for _array_element _output_get
    (if (Utilities|Enum|Equal(Enum) (Variables|/Game/Building/BP_Building.BP_Building_C|GetDifficulty _array_element) (Variables|Default|GetDifficulty))
      (Utilities|Array|Add (Variables|Default|GetDifficultyBuildings) _array_element) ; Stores only the buildings for the selected game mode
    )))

(fn ConstructionScript)